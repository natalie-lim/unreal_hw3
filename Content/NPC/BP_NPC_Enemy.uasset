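; Enemy NPC that opens a dialogue on first player overlap, then becomes a combatant and owns the fight's health and end-game UI.
; After first contact, Tick loops it along the BP_SplinePath spline, while later overlaps set the blackboard attack state and punch the player.
; Player projectiles lower NPC health; FireAtPlayer spawns aimed enemy projectiles.
; ApplyDamage tracks player health separately from punch damage, and EndGame pauses with a win or lose screen.
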(event `self.ReceiveBeginPlay`
  (bind _returnvalue (`GameplayStatics.GetActorOfClass` "/Game/FirstPerson/Blueprints/BP_SplinePath.BP_SplinePath_C"))
  (set `self.SplineReference` (`/Game/FirstPerson/Blueprints/BP_SplinePath.Spline` _returnvalue))
  (bind _returnvalue_2 (`|CreateWidget` "/Game/Widgets/WBP_BeginScreen.WBP_BeginScreen_C"))
  (bind _output_get (set `self.StartWidget` _returnvalue_2))
  (`UserWidget.AddToViewport` _output_get 0)
  (bind _returnvalue_3 (`|CreateWidget` "/Game/Widgets/WBP_FightingWidgets.WBP_FightingWidgets_C" null null))
  (set `/Game/Widgets/WBP_FightingWidgets.OwningActorRef` self _returnvalue_3)
  (bind _output_get_2 (set `self.HealthWidgetRef` _returnvalue_3))
  (`UserWidget.AddToViewport` _output_get_2 0))

(event `self.TriggerBox.OnComponentBeginOverlap`
  (params (OverlappedComponent :type "PrimitiveComponent Object Reference") (OtherActor :type "Actor Object Reference") (OtherComp :type "PrimitiveComponent Object Reference") (OtherBodyIndex :type Integer) (bFromSweep :type Boolean) (SweepResult :type "HitResult Structure (by ref)"))
  (cast `/Game/FirstPerson/Blueprints/BP_Projectile` OtherActor
    (:`then`
      (`KismetSystemLibrary.PrintString` "enemy hit by bullet")
      (bind _output_get (set `self.NPCHealth` (- (`self.NPCHealth`) 1.0)))
      (`/Game/Widgets/WBP_FightingWidgets.UpdateEnemyHealth` (`self.HealthWidgetRef`) _output_get))
    (:`CastFailed`
      (bind _asbp_first_person_character (cast `/Game/FirstPerson/Blueprints/BP_FirstPersonCharacter` OtherActor))
      (if (`self.bHasNotTalked`)
        (`Widget.RemoveFromParent` (`self.StartWidget`))
        (bind _returnvalue (`|CreateWidget` "/Game/Widgets/WBP_DialogueBox.WBP_DialogueBox_C" null (struct) null))
        (set `/Game/Widgets/WBP_DialogueBox.DialogueTable` (`self.DialogueTable`) _returnvalue)
        (bind _output_get_2 (set `self.DialogueWidget` _returnvalue))
        (set `/Game/Widgets/WBP_DialogueBox.TargetNPC` self _output_get_2)
        (`UserWidget.AddToViewport` _returnvalue 0)
        (bind _returnvalue_2 (`InputDeviceLibrary.GetPlayerControllerFromInputDevice` (struct)))
        (`self.DisableInput` _asbp_first_person_character _returnvalue_2)
        (`KismetSystemLibrary.Delay` 1.0)
        (cast `/Game/Characters/Mannequins/Anims/Unarmed/ABP_Unarmed` (`SkeletalMeshComponent.GetAnimInstance` (`self.Mesh`)))
        (set `self.bHasNotTalked` false)
        (`KismetSystemLibrary.Delay` 0.2)
        (else
          (bind _asbp_npc_aicontroller (cast `/Game/NPC/BP_NPC_AIController` (`self.GetController`)))
          (`BlackboardComponent.SetValueAsInt` (`AIController.Blackboard` _asbp_npc_aicontroller) "CurrentState" 1)
          (`KismetSystemLibrary.PrintString` "enemy punches you")
          (bind _output_get_3 (set `self.CurrentHealth` (- (`self.CurrentHealth`) 4.0)))
          (`/Game/Widgets/WBP_FightingWidgets.UpdateHealth` (`self.HealthWidgetRef`) _output_get_3))))))

(event `FireAtPlayer`
  (bind _returnvalue (`self.K2_GetActorLocation`))
  (bind _asbp_first_person_character (cast `/Game/FirstPerson/Blueprints/BP_FirstPersonCharacter` (`GameplayStatics.GetPlayerCharacter` 0)))
  (`SkeletalMeshComponent.PlayAnimation` (`self.Mesh`) "/Game/Characters/Mannequins/Anims/Rifle/AIM/AO_Rifle.AO_Rifle" true)
  (bind _returnvalue_2 (`KismetMathLibrary.FindLookAtRotation` _returnvalue (`self.K2_GetActorLocation` _asbp_first_person_character)))
  (`self.K2_SetActorRotation` _returnvalue_2)
  (`|SpawnActorFromClass` "/Game/FirstPerson/Blueprints/BP_Projectile_Enemy.BP_Projectile_Enemy_C" (`KismetMathLibrary.MakeTransform` _returnvalue _returnvalue_2) "Undefined" "MultiplyWithRoot" null null)
  (`SkeletalMeshComponent.PlayAnimation` (`self.Mesh`) "/Game/Characters/Mannequins/Anims/Unarmed/BS_Idle_Walk_Run.BS_Idle_Walk_Run" false))

(event `self.ReceiveTick`
  (params (DeltaSeconds :type "Float (single-precision)"))
  (bind _splinereference (`self.SplineReference`))
  (if (not (`self.bHasNotTalked`))
    (bind _output_get (set `self.DistanceAlongSpline` (mod (+ (`self.DistanceAlongSpline`) (* 250.0 DeltaSeconds)) (`SplineComponent.GetSplineLength` _splinereference))))
    (`self.K2_SetActorLocation` (`SplineComponent.GetLocationAtDistanceAlongSpline` _splinereference _output_get "World"))))

(event `/Game/FirstPerson/Blueprints/BPI_TakeDamage.ApplyDamage`
  (params (DamageAmount :type "Float (double-precision)"))
  (bind _output_get (set `self.PersonHealth` (- (`self.PersonHealth`) DamageAmount)))
  (`/Game/Widgets/WBP_FightingWidgets.UpdateHealth` (`self.HealthWidgetRef`) _output_get)
  (`KismetSystemLibrary.PrintString` "damage from enemy bullet :("))

(event `EndGame`
  (params (YouWon :type Boolean))
  (`Widget.RemoveFromParent` (`self.HealthWidgetRef`))
  (set `PlayerController.bShowMouseCursor` true (`PlayerState.GetPlayerController` (`GameplayStatics.GetPlayerState` 0)))
  (`GameplayStatics.SetGamePaused` true)
  (if YouWon
    (bind _returnvalue (`|CreateWidget` "/Game/Widgets/WBP_YouWin.WBP_YouWin_C"))
    (`UserWidget.AddToViewport` _returnvalue 0)
    (else
      (bind _returnvalue_2 (`|CreateWidget` "/Game/Widgets/WBP_EnemyWin.WBP_EnemyWin_C"))
      (`UserWidget.AddToViewport` _returnvalue_2 0))))

(fn `UserConstructionScript`)