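; AI controller for NPC enemies that drives their behavior state from distance to the player.
; On possess it runs the NPC behavior tree, sets up its blackboard and stores the player character as TargetActor.
; Every tick, for a possessed BP_NPC_Enemy, it writes an integer CurrentState to the blackboard, switching between two values at a fixed distance threshold from the player.
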(event `self.ReceivePossess`
  (params (PossessedPawn :type "Pawn Object Reference"))
  (`self.RunBehaviorTree` "/Game/NPC/BT_NPCBehavior.BT_NPCBehavior")
  (bind _blackboardcomponent (`self.UseBlackboard` "/Game/NPC/BB_NPCBehavior.BB_NPCBehavior"))
  (`BlackboardComponent.SetValueAsObject` _blackboardcomponent (`KismetStringLibrary.Conv_StringToName` "TargetActor") (`GameplayStatics.GetPlayerCharacter` 0)))

(event `self.ReceiveTick`
  (params (DeltaSeconds :type "Float (single-precision)"))
  (bind _returnvalue (`KismetStringLibrary.Conv_StringToName` "CurrentState"))
  (bind _asbp_npc_enemy (cast `/Game/NPC/BP_NPC_Enemy` (stale `self.ReceivePossess` PossessedPawn)))
  (if (> (`self.GetDistanceTo` (`GameplayStatics.GetPlayerCharacter` 0) _asbp_npc_enemy) 300.0)
    (`BlackboardComponent.SetValueAsInt` (stale `self.ReceivePossess` _blackboardcomponent) _returnvalue 2)
    (else
      (`BlackboardComponent.SetValueAsInt` (stale `self.ReceivePossess` _blackboardcomponent) _returnvalue 1))))

(fn `UserConstructionScript`)